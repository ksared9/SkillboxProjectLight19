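; BP_Button is a switch Blueprint that toggles lamps in the level when its Switch event is called.
; Each call refreshes TargetLamps with GetAllActorsOfClass on BP_Light, then a Sequence drives three FlipFlops for the first three entries.
; Each FlipFlop alternates its lamp's PointLight intensity between lit and zero, relying on fixed array indices rather than a loop.
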(event EventBeginPlay)

(event Collision|EventActorBeginOverlap
  (params (OtherActor :type Actor%20Object%20Reference)))

(event EventTick
  (params (DeltaSeconds :type Float%20%28single-precision%29)))

(event EventSwitch
  (bind _outactors (Actor|GetAllActorsOfClass "/Game/Blueprints/BP_Light.BP_Light_C"))
  (bind _output_get (Variables|Default|SetTargetLamps _outactors))
  (Utilities|FlowControl|Sequence
    (:then_0
      (Utilities|FlowControl|FlipFlop
        (:A
          (Rendering|Components|Light|SetIntensity (Variables|/Game/Blueprints/BP_Light.BP_Light_C|GetPointLight (Utilities|Array|Get(acopy) _output_get)) 5e+02))
        (:B
          (Rendering|Components|Light|SetIntensity (Variables|/Game/Blueprints/BP_Light.BP_Light_C|GetPointLight (Utilities|Array|Get(acopy) _output_get)) 0.0))))
    (:then_1
      (Utilities|FlowControl|FlipFlop
        (:A
          (Rendering|Components|Light|SetIntensity (Variables|/Game/Blueprints/BP_Light.BP_Light_C|GetPointLight (Utilities|Array|Get(acopy) _output_get 1)) 5e+02))
        (:B
          (Rendering|Components|Light|SetIntensity (Variables|/Game/Blueprints/BP_Light.BP_Light_C|GetPointLight (Utilities|Array|Get(acopy) _output_get 1)) 0.0))))
    (:then_2
      (Utilities|FlowControl|FlipFlop
        (:A
          (Rendering|Components|Light|SetIntensity (Variables|/Game/Blueprints/BP_Light.BP_Light_C|GetPointLight (Utilities|Array|Get(acopy) _output_get 2)) 5e+02))
        (:B
          (Rendering|Components|Light|SetIntensity (Variables|/Game/Blueprints/BP_Light.BP_Light_C|GetPointLight (Utilities|Array|Get(acopy) _output_get 2)) 0.0))))))

(fn ConstructionScript)